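; Actor component for RTS buildings that manages health, housing and unit production.
; Owner damage updates an added health bar, destroying the building at zero and repairing it at full health, with housing resources adjusted accordingly.
; A self-recalling queue cycle charges the player, waits, then spawns units at random goal-location components, dropping orders lacking funds or housing.
; Helpers find the closest goal point and tally queued units by type.
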(event `self.ReceiveBeginPlay`
  (`|ExecutionSequence`
    (:`then_0`
      (bind _returnvalue (`|AddComponentByClass` (`self.GetOwner`) "/Game/RTSGame/Core/Common/BP_HealthBarWidgetComponent.BP_HealthBarWidgetComponent_C" false (`KismetMathLibrary.MakeTransform` (`self.HealthBarRelativeLocation`))))
      (`WidgetComponent.SetDrawSize` _returnvalue (`self.HealthBarDrawSize`))
      (`self.UpdateHealthBar`)
      (bind _asbp_building (cast `/Game/RTSGame/Core/Building/BP_Building` (`self.GetOwner`)))
      (if (`self.IsDestroyed`)
        (`/Game/RTSGame/Core/Building/BP_Building.DestroyBuilding` _asbp_building null null)
        (else
          (`/Game/RTSGame/Core/Building/BP_Building.RepairBuilding` _asbp_building null null)
          (bind _aspc_rtsgame (cast `/Game/RTSGame/Core/Player/PC_RTSGame` (`GameplayStatics.GetPlayerController` 0)))
          (`/Game/RTSGame/Core/Player/PC_RTSGame.ReceiveResources` _aspc_rtsgame "NewEnumerator2" (`self.HousingValue`)))))
    (:`then_1`
      (add `Actor.OnTakeAnyDamage` (`self.GetOwner`) (`|CreateDelegate` :!event `OnOwnerTakeAnyDamage`)))))

(event `OnOwnerTakeAnyDamage`
  (params (DamagedActor :type "Actor Object Reference") (Damage :type "Float (single-precision)") (DamageType :type "DamageType Object Reference") (InstigatedBy :type "Controller Object Reference") (DamageCauser :type "Actor Object Reference"))
  (set `self.Health` (`KismetMathLibrary.FMin` (`KismetMathLibrary.FMax` (- (`self.Health`) Damage)) (`self.HealthMax`)))
  (`self.UpdateHealthBar`)
  (bind _asbp_building (cast `/Game/RTSGame/Core/Building/BP_Building` (`self.GetOwner`)))
  (if (<= (`self.Health`) 0.0)
    (if (not (`self.IsDestroyed`))
      (set `self.IsDestroyed` true)
      (`/Game/RTSGame/Core/Building/BP_Building.DestroyBuilding` _asbp_building null null)
      (`self.OnBuildingDestroyed` (`self.GetOwner`))
      (bind _aspc_rtsgame (cast `/Game/RTSGame/Core/Player/PC_RTSGame` (`GameplayStatics.GetPlayerController` 0)))
      (`/Game/RTSGame/Core/Player/PC_RTSGame.ReceiveResources` _aspc_rtsgame "NewEnumerator2" (* (`self.HousingValue`) -1)))
    (elif (and (>= (`self.Health`) (`self.HealthMax`)) (`self.IsDestroyed`))
      (set `self.IsDestroyed` false)
      (`/Game/RTSGame/Core/Building/BP_Building.RepairBuilding` _asbp_building null null)
      (bind _aspc_rtsgame_2 (cast `/Game/RTSGame/Core/Player/PC_RTSGame` (`GameplayStatics.GetPlayerController` 0)))
      (`/Game/RTSGame/Core/Player/PC_RTSGame.ReceiveResources` _aspc_rtsgame_2 "NewEnumerator2" (`self.HousingValue`)))))

(event `ProduceUnit`
  (params (UnitToProduce :type "/Game/RTSGame/Core/Unit/BP_Unit Class Reference"))
  (`KismetArrayLibrary.Array_Add` (`self.UnitProductionQueue`) UnitToProduce)
  (if (not (`self.IsProducingUnits`))
    (`self.ProducingUnitsCycle`)))

(event `ProducingUnitsCycle`
  (bind _output (`|GetArrayItem` (`self.UnitProductionQueue`)))
  (bind (_price _time_to_produce) (`self.GetUnitPriceAndTime` _output))
  (if (>= (`KismetArrayLibrary.Array_Length` (`self.UnitProductionQueue`)) 1)
    (set `self.IsProducingUnits` true)
    (bind _aspc_rtsgame (cast `/Game/RTSGame/Core/Player/PC_RTSGame` (`GameplayStatics.GetPlayerController` 0)))
    (bind _storedresources (`/Game/RTSGame/Core/Player/PC_RTSGame.StoredResources` _aspc_rtsgame))
    (if (and (>= _price 0) (<= _price (`BlueprintMapLibrary.Map_Find` _storedresources "NewEnumerator1")) (> (`BlueprintMapLibrary.Map_Find` _storedresources "NewEnumerator2") 0))
      (`/Game/RTSGame/Core/Player/PC_RTSGame.ReceiveResources` _aspc_rtsgame "NewEnumerator1" (* _price -1))
      (`KismetSystemLibrary.Delay` _time_to_produce)
      (bind _returnvalue (`|SpawnActorFromClass` _output (`KismetMathLibrary.MakeTransform` (`SceneComponent.K2_GetComponentLocation` (`KismetArrayLibrary.Array_Random` (`Actor.K2_GetComponentsByClass` (`self.GetOwner`) "/Game/RTSGame/Core/Building/BP_GoalLocationComponent.BP_GoalLocationComponent_C")))) "AdjustIfPossibleButAlwaysSpawn" "MultiplyWithRoot" null null))
      (`self.OnUnitCreated` _returnvalue))
    (`KismetArrayLibrary.Array_Remove` (`self.UnitProductionQueue`))
    (`self.ProducingUnitsCycle`)
    (else
      (set `self.IsProducingUnits` false))))

(fn `Get Suitable Location`
  (params (ObjLocation :type "Vector Structure"))
  (returns (SuitableLocationRef :type "/Game/RTSGame/Core/Building/BP_GoalLocationComponent Object Reference"))
  (locals (ClosestPoint :type "/Game/RTSGame/Core/Building/BP_GoalLocationComponent Object Reference"))
  (bind _returnvalue (`Actor.K2_GetComponentsByClass` (`self.GetOwner`) "/Game/RTSGame/Core/Building/BP_GoalLocationComponent.BP_GoalLocationComponent_C"))
  (if (`KismetArrayLibrary.Array_IsNotEmpty` _returnvalue)
    (set `local.ClosestPoint` (`|GetArrayItem` _returnvalue))
    (for _array_element _returnvalue
      (if (< (`KismetMathLibrary.Vector_Distance` (`SceneComponent.K2_GetComponentLocation` _array_element) ObjLocation) (`KismetMathLibrary.Vector_Distance` (`SceneComponent.K2_GetComponentLocation` (`local.ClosestPoint`)) ObjLocation))
        (set `local.ClosestPoint` _array_element)))
    (return (`local.ClosestPoint`))
    (else
      (return null))))

(fn `GetUnitPriceAndTime`
  (params (UnitToProduce :type "/Game/RTSGame/Core/Unit/BP_Unit Class Reference"))
  (returns (Price :type Integer) (`Time to Produce` :type "Float (double-precision)"))
  (for _array_element (`self.UnitProductionInfo`)
    (if (== (break `/Game/RTSGame/Core/Building/S_UnitProducionInfo` _array_element) UnitToProduce)
      (return (`.Price_7_64264AA247A25474185843918D6842F3` (break `/Game/RTSGame/Core/Building/S_UnitProducionInfo` _array_element)) (`.TimeToProduce_8_2B9293FB4D6F4C6D9372E9995DF1D1C6` (break `/Game/RTSGame/Core/Building/S_UnitProducionInfo` _array_element)))))
  (return -1 -1.0))

(fn `GetUnitQueue`
  (returns (UnitQueue :type "Map of /Game/RTSGame/Core/Unit/BP_Unit Class Reference to Integer"))
  (locals (NewLocalVar :type "Map of /Game/RTSGame/Core/Unit/BP_Unit Class Reference to Integer"))
  (bind _newlocalvar (`local.NewLocalVar`))
  (for _array_element (`self.UnitProductionQueue`)
    (bind (_value _returnvalue) (`BlueprintMapLibrary.Map_Find` (`local.NewLocalVar`) _array_element))
    (if _returnvalue
      (`BlueprintMapLibrary.Map_Add` _newlocalvar _array_element (+ _value 1))
      (else
        (`BlueprintMapLibrary.Map_Add` _newlocalvar _array_element 1))))
  (return (`local.NewLocalVar`)))

(fn `UpdateHealthBar`
  (bind _returnvalue (`Actor.GetComponentByClass` (`self.GetOwner`) "/Game/RTSGame/Core/Common/BP_HealthBarWidgetComponent.BP_HealthBarWidgetComponent_C"))
  (`/Engine/EditorBlueprintResources/StandardMacros.IsValid` _returnvalue
    (:`Is Valid`
      (`/Game/RTSGame/Core/Common/BP_HealthBarWidgetComponent.UpdateHealthBar` _returnvalue (/ (`self.Health`) (`self.HealthMax`))))
    (:`Is Not Valid`
      (`KismetSystemLibrary.PrintString` "Building Component: no healthbar component valid"))))