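; BP_Building is a building actor for the RTS game, handling selection, housing resource loss and intact/destroyed visuals.
; Clicking adds it to PC_RTSGame's selection list and shows its BPSelectionComponent decal, which SelectThis and DeselectThis also toggle.
; BPBuildingComponent supplies team attitude and state; its destruction event and actor Destroyed both deduct HousingValue through the player controller unless IsDestroyed is set.
; DestroyBuilding and RepairBuilding swap visibility between two supplied objects.
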(event `self.ReceiveActorOnClicked`
  (params (ButtonPressed :type "Key Structure"))
  (`self.BuildingClicked`))

(event `BuildingClicked`
  (`|ExecutionSequence`
    (:`then_0`
      (bind _aspc_rtsgame (cast `/Game/RTSGame/Core/Player/PC_RTSGame` (`GameplayStatics.GetPlayerController` 0)))
      (`/Game/RTSGame/Core/Player/PC_RTSGame.AddActorSelectedToList` _aspc_rtsgame self))
    (:`then_1`
      (`/Game/RTSGame/Core/Common/BP_SelectionComponent.ShowSelectionDecal` (`self.BP_SelectionComponent`)))))

(event `self.BP_BuildingComponent.OnBuildingDestroyed`
  (params (ActorDestroyed :type "Actor Object Reference"))
  (bind _bp_buildingcomponent (`self.BP_BuildingComponent`))
  (if (not (`/Game/RTSGame/Core/Building/BP_BuildingComponent.IsDestroyed` _bp_buildingcomponent)) :!label _label
    (bind _aspc_rtsgame (cast `/Game/RTSGame/Core/Player/PC_RTSGame` (`GameplayStatics.GetPlayerController` 0)))
    (`/Game/RTSGame/Core/Player/PC_RTSGame.ReceiveResources` _aspc_rtsgame "NewEnumerator2" (* (`/Game/RTSGame/Core/Building/BP_BuildingComponent.HousingValue` _bp_buildingcomponent) -1))))

(event `self.ReceiveDestroyed`
  (goto _label))

(event `/Game/RTSGame/Core/Common/BPI_SelectionEvents.SelectThis`
  (`/Game/RTSGame/Core/Common/BP_SelectionComponent.ShowSelectionDecal` (`self.BP_SelectionComponent`)))

(event `/Game/RTSGame/Core/Common/BPI_SelectionEvents.DeselectThis`
  (`/Game/RTSGame/Core/Common/BP_SelectionComponent.HideSelectionDecal` (`self.BP_SelectionComponent`)))

(fn `DestroyBuilding`
  (params (ObjectToHide :type "SceneComponent Object Reference") (ObjectToShow :type "SceneComponent Object Reference"))
  (`SceneComponent.SetHiddenInGame` ObjectToHide true false)
  (`SceneComponent.SetHiddenInGame` ObjectToShow false false))

(fn `GetTeamAttitude`
  (returns (TeamAttitude :type "ETeamAttitude Enum"))
  (return (`/Game/RTSGame/Core/Building/BP_BuildingComponent.TeamAttitude` (`self.BP_BuildingComponent`))))

(fn `RepairBuilding`
  (params (ObjectToHide :type "SceneComponent Object Reference") (ObjectToShow :type "SceneComponent Object Reference"))
  (`SceneComponent.SetHiddenInGame` ObjectToHide true false)
  (`SceneComponent.SetHiddenInGame` ObjectToShow false false))

(fn `UserConstructionScript`)