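; BP_HealingZone is an RTS area actor that periodically heals units of a matching team attitude within a radius.
; On BeginPlay, a looping timer runs a sphere overlap against Pawns at the set interval, drawing a debug sphere each time.
; Pawns with a BP_UnitComponent whose TeamAttitude matches the zone's receive negative damage through ApplyDamage, so healing reuses the damage pipeline.
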(event `self.ReceiveBeginPlay`
  (`KismetSystemLibrary.K2_SetTimerDelegate` (delegate `SpawnOverlapSphere`) (`self.Interval`) true))

(event `SpawnOverlapSphere`
  (bind _returnvalue (`self.K2_GetActorLocation`))
  (bind _radius (`self.Radius`))
  (`KismetSystemLibrary.DrawDebugSphere` _returnvalue _radius)
  (bind _outactors (`KismetSystemLibrary.SphereOverlapActors` _returnvalue _radius (`|MakeArray` "ObjectTypeQuery3" :!type "EObjectTypeQuery Enum")))
  (for _array_element _outactors
    (bind _returnvalue_2 (`self.GetComponentByClass` _array_element "/Game/RTSGame/Core/Unit/BP_UnitComponent.BP_UnitComponent_C"))
    (`/Engine/EditorBlueprintResources/StandardMacros.IsValid` _returnvalue_2
      (:`Is Valid`
        (if (`|EnumEquality` (`/Game/RTSGame/Core/Unit/BP_UnitComponent.TeamAttitude` _returnvalue_2) (`self.TeamAttitude`))
          (`GameplayStatics.ApplyDamage` _array_element (* (`self.HPAdded`) -1.0)))))))

(fn `UserConstructionScript`)