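; Actor component for RTS units that manages health, team attitude, click selection and unit state.
; On BeginPlay it adds a team-colored health bar to its owner and binds click and damage events, with friendly clicks adding to the player controller's selection.
; Damage updates the bar, broadcasts HP changes and sets a Scout low-health blackboard flag that clears only at full health.
; Death destroys the owner, updates selection and HUD, and refunds the resource friendly units take on spawn.
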(event `self.ReceiveBeginPlay`
  (`|ExecutionSequence`
    (:`then_0`
      (bind _returnvalue (`|AddComponentByClass` (`self.GetOwner`) "/Game/RTSGame/Core/Common/BP_HealthBarWidgetComponent.BP_HealthBarWidgetComponent_C" false (`KismetMathLibrary.MakeTransform` (`self.HealthBarRelativeLocation`))))
      (`WidgetComponent.SetDrawSize` _returnvalue (`self.HealthBarDrawSize`))
      (`/Game/RTSGame/Core/Common/BP_HealthBarWidgetComponent.UpdateHealthBarColor` _returnvalue (select `ETeamAttitude` (`self.TeamAttitude`) :`Friendly` (struct :`G` 0.274931 :`B` 0.755208 :`A` 1.0) :`Neutral` (struct :`R` 0.942708 :`G` 0.901852 :`A` 1.0) :`Hostile` (struct :`R` 1.0 :`G` 0.030547 :`A` 1.0) :!type "LinearColor Structure"))
      (`self.UpdateHealthBar`))
    (:`then_1`
      (add `Actor.OnClicked` (`self.GetOwner`) (`|CreateDelegate` :!event `OnOwnerClicked`))
      (add `Actor.OnTakeAnyDamage` (`self.GetOwner`) (`|CreateDelegate` :!event `OnOwnerTakeAnyDamage`))
      (if (`|EnumEquality` (`self.TeamAttitude`) "Friendly")
        (bind _aspc_rtsgame (cast `/Game/RTSGame/Core/Player/PC_RTSGame` (`GameplayStatics.GetPlayerController` 0)))
        (`/Game/RTSGame/Core/Player/PC_RTSGame.ReceiveResources` _aspc_rtsgame "NewEnumerator2" -1)))))

(event `OnOwnerClicked`
  (params (TouchedActor :type "Actor Object Reference") (ButtonPressed :type "Key Structure" :default "None"))
  (if (`|EnumEquality` (`self.TeamAttitude`) "Friendly")
    (`self.AddUnitToSelectionList`)))

(event `AddUnitToSelectionList`
  (clear `self.OnHPChanged`)
  (bind _aspc_rtsgame (cast `/Game/RTSGame/Core/Player/PC_RTSGame` (`GameplayStatics.GetPlayerController` 0)))
  (`/Game/RTSGame/Core/Player/PC_RTSGame.AddActorSelectedToList` _aspc_rtsgame (`self.GetOwner`)))

(event `OnOwnerTakeAnyDamage`
  (params (DamagedActor :type "Actor Object Reference") (Damage :type "Float (single-precision)") (DamageType :type "DamageType Object Reference") (InstigatedBy :type "Controller Object Reference") (DamageCauser :type "Actor Object Reference"))
  (bind _returnvalue (`self.GetOwner`))
  (bind _healthmax (`self.HealthMax`))
  (bind _output_get (set `self.Health` (`KismetMathLibrary.FMin` (`KismetMathLibrary.FMax` (- (`self.Health`) Damage)) _healthmax)))
  (if (< _output_get (* _healthmax 0.3))
    (bind _asbp_scout (cast `/Game/RTSGame/Units/Hostile/BP_Scout` (`self.GetOwner`))
      (:`then`
        (`BlackboardComponent.SetValueAsBool` (`AIBlueprintHelperLibrary.GetBlackboard` (`AIBlueprintHelperLibrary.GetAIController` _asbp_scout)) "isLowHealth" true))
      (:`CastFailed`
        _))
    (elif (== _output_get _healthmax)
      (bind _asbp_scout_2 (cast `/Game/RTSGame/Units/Hostile/BP_Scout` (`self.GetOwner`))
        (:`then`
          (`BlackboardComponent.SetValueAsBool` (`AIBlueprintHelperLibrary.GetBlackboard` (`AIBlueprintHelperLibrary.GetAIController` _asbp_scout_2)) "isLowHealth" false))
        (:`CastFailed`
          _))))
  (`self.UpdateHealthBar`)
  (if (<= _output_get 0.0)
    (clear `self.OnHPChanged`)
    (bind _aspc_rtsgame (cast `/Game/RTSGame/Core/Player/PC_RTSGame` (`GameplayStatics.GetPlayerController` 0)))
    (bind _selectedactors (`/Game/RTSGame/Core/Player/PC_RTSGame.SelectedActors` _aspc_rtsgame))
    (`KismetArrayLibrary.Array_RemoveItem` _selectedactors _returnvalue)
    (`Actor.K2_DestroyActor` _returnvalue)
    (bind _asbp_hud (cast `/Game/RTSGame/Core/Player/BP_HUD` (`PlayerController.GetHUD` (`GameplayStatics.GetPlayerController` 0))))
    (`/Game/RTSGame/UI/HUD/WBP_HUD.UpdateInfoPanel` (`/Game/RTSGame/Core/Player/BP_HUD.HUDWidgetReference` _asbp_hud) _selectedactors)
    (if (`|EnumEquality` (`self.TeamAttitude`) "Friendly")
      (bind _aspc_rtsgame_2 (cast `/Game/RTSGame/Core/Player/PC_RTSGame` (`GameplayStatics.GetPlayerController` 0)))
      (`/Game/RTSGame/Core/Player/PC_RTSGame.ReceiveResources` _aspc_rtsgame_2 "NewEnumerator2" 1))
    (else
      (bind _asbp_unit (cast `/Game/RTSGame/Core/Unit/BP_Unit` (`self.GetOwner`)))
      (`self.OnHPChanged` (`self.Health`) _asbp_unit))))

(fn `HandleNewUnitState`
  (params (NewUnitState :type "/Game/RTSGame/Core/Unit/E_UnitAnimationStates Enum" :default "NewEnumerator0"))
  (if (not (`|EnumEquality` (`self.UnitState`) NewUnitState))
    (bind _output_get (set `self.UnitState` NewUnitState))
    (`self.OnEnterNewState` _output_get)
    (if (`|EnumEquality` _output_get "NewEnumerator1")
      _)))

(fn `UpdateHealthBar`
  (bind _returnvalue (`Actor.GetComponentByClass` (`self.GetOwner`) "/Game/RTSGame/Core/Common/BP_HealthBarWidgetComponent.BP_HealthBarWidgetComponent_C"))
  (`/Engine/EditorBlueprintResources/StandardMacros.IsValid` _returnvalue
    (:`Is Valid`
      (`/Game/RTSGame/Core/Common/BP_HealthBarWidgetComponent.UpdateHealthBar` _returnvalue (/ (`self.Health`) (`self.HealthMax`))))
    (:`Is Not Valid`
      (`KismetSystemLibrary.PrintString` "Unit Component: no healthbar component valid"))))