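; BP_ResourceGatherIndicator is a short-lived actor in the RTS game's resource system that, per its name, signals a resource gather with a rising mesh.
; The construction script assigns MeshToUse to ResourceMesh.
; On BeginPlay, the UpwardsAnimation timeline drives the mesh's relative Z up to MaxUpwardsDistance, then the actor destroys itself.
; A play-rate change for the timeline is present but unconnected.
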(event `self.ReceiveBeginPlay`
  (bind (_direction _zvaluealpha) (`Timeline|UpwardsAnimation`)
    (:`Update`
      (`SceneComponent.K2_SetRelativeLocation` (`self.ResourceMesh`) (`KismetMathLibrary.MakeVector` 0.0 0.0 (* _zvaluealpha (`self.MaxUpwardsDistance`))) false false))
    (:`Finished`
      (`self.K2_DestroyActor`))))

(fn `UserConstructionScript`
  (`StaticMeshComponent.SetStaticMesh` (`self.ResourceMesh`) (`self.MeshToUse`)))