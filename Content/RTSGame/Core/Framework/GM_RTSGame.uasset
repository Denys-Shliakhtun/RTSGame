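; RTS game mode that decides win and loss, showing the matching screen and pausing the game.
; PreBindObjects, not called from BeginPlay here, binds to town hall, worker and enemy spawner events, including units created by friendly town halls.
; Loss requires no workers and no intact friendly town hall.
; Kills decrement per-class EnemiesToKillToWin counts, refreshing HUD goals for Mongols, Barbarians and Guardians until all reach zero.
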(event `self.ReceiveBeginPlay`)

(event `PreBindObjects`
  (bind _outactors (`GameplayStatics.GetAllActorsOfClass` "/Game/RTSGame/Buildings/BP_Townhall.BP_Townhall_C"))
  (bind _output_get (set `self.TownHalls` _outactors))
  (for _array_element _output_get
    (add `/Game/RTSGame/Core/Building/BP_BuildingComponent.OnBuildingDestroyed` (`self.GetComponentByClass` _array_element "/Game/RTSGame/Core/Building/BP_BuildingComponent.BP_BuildingComponent_C") (`|CreateDelegate` :!event `OnImportantObjectDestroyed`)))
  (bind _outactors_2 (`GameplayStatics.GetAllActorsOfClass` "/Game/RTSGame/Units/Friendly/BP_Worker.BP_Worker_C"))
  (for _array_element_2 _outactors_2
    (add `self.OnDestroyed` _array_element_2 (`|CreateDelegate` :!event `OnImportantObjectDestroyed`)))
  (for _array_element_3 (`self.TownHalls`)
    (bind _returnvalue (`self.GetComponentByClass` _array_element_3 "/Game/RTSGame/Core/Building/BP_BuildingComponent.BP_BuildingComponent_C"))
    (if (`|EnumEquality` (`/Game/RTSGame/Core/Building/BP_BuildingComponent.TeamAttitude` _returnvalue) "Friendly")
      (add `/Game/RTSGame/Core/Building/BP_BuildingComponent.OnUnitCreated` _returnvalue (delegate `CustomEvent`))))
  (`KismetSystemLibrary.Delay` 0.2)
  (bind _outactors_3 (`GameplayStatics.GetAllActorsOfClass` "/Game/RTSGame/Core/Enemy/BP_EnemySpawner.BP_EnemySpawner_C"))
  (for _array_element_4 _outactors_3
    (add `/Game/RTSGame/Core/Enemy/BP_EnemySpawner.EnemyDestroyed` _array_element_4 (`|CreateDelegate` :!event `OnEnemyDestroyed`)))
  (`KismetSystemLibrary.Delay` 0.2)
  (`self.UpdateCurrentGoals`))

(event `CustomEvent`
  (params (Unit :type "Actor Object Reference"))
  (add `self.OnDestroyed` Unit (`|CreateDelegate` :!event `OnImportantObjectDestroyed`)))

(event `OnImportantObjectDestroyed` :!signature `self.OnDestroyed`
  (params (ActorDestroyed :type "Actor Object Reference"))
  (`KismetSystemLibrary.Delay` 0.2)
  (if (not (or (`self.DoesPlayerHaveWorkers`) (`self.DoesPlayerTownExist`)))
    (`self.LoseTheGame`)))

(event `LoseTheGame`
  (bind _returnvalue (`|CreateWidget` "/Game/RTSGame/UI/Menus/WBP_LoseScreen.WBP_LoseScreen_C"))
  (`UserWidget.AddToViewport` _returnvalue 0)
  (`GameplayStatics.SetGamePaused` true))

(event `OnEnemyDestroyed`
  (params (Unit :type "Actor Object Reference"))
  (bind _returnvalue (`GameplayStatics.GetObjectClass` Unit))
  (bind _enemiestokilltowin (`self.EnemiesToKillToWin`))
  (bind (_value _returnvalue_2) (`BlueprintMapLibrary.Map_Find` _enemiestokilltowin _returnvalue))
  (if (and _returnvalue_2 (> _value 0))
    (`BlueprintMapLibrary.Map_Add` _enemiestokilltowin _returnvalue (- _value 1))
    (`self.UpdateCurrentGoals`)
    (if (`self.HasPlayerWon`)
      (`self.WinTheGame`))))

(event `WinTheGame`
  (bind _returnvalue (`|CreateWidget` "/Game/RTSGame/UI/Menus/WBP_WinScreen.WBP_WinScreen_C"))
  (`UserWidget.AddToViewport` _returnvalue 0)
  (`GameplayStatics.SetGamePaused` true))

(fn `DoesPlayerHaveWorkers`
  (returns (DoWorkersExist :type Boolean))
  (bind _outactors (`GameplayStatics.GetAllActorsOfClass` "/Game/RTSGame/Units/Friendly/BP_Worker.BP_Worker_C"))
  (return (`KismetArrayLibrary.Array_IsNotEmpty` _outactors)))

(fn `DoesPlayerTownExist`
  (returns (DoesTownExist :type Boolean))
  (for _array_element (`self.TownHalls`)
    (bind _returnvalue (`self.GetComponentByClass` _array_element "/Game/RTSGame/Core/Building/BP_BuildingComponent.BP_BuildingComponent_C"))
    (if (and (`|EnumEquality` (`/Game/RTSGame/Core/Building/BP_BuildingComponent.TeamAttitude` _returnvalue) "Friendly") (not (`/Game/RTSGame/Core/Building/BP_BuildingComponent.IsDestroyed` _returnvalue)))
      (return true)))
  (return false))

(fn `GetPlayerTown`
  (returns (PlayerTownHall :type "Actor Object Reference"))
  (locals (FoundIndex :type Integer))
  (for _array_element (`self.TownHalls`)
    (bind _returnvalue (`KismetArrayLibrary.Array_Find` (`Actor.Tags` _array_element) "Player"))
    (if (>= _returnvalue 0)
      (set `local.FoundIndex` _returnvalue)
      (break)))
  (return (`|GetArrayItem` (`self.TownHalls`) (`local.FoundIndex`))))

(fn `HasPlayerWon`
  (returns (HasWon :type Boolean))
  (bind _values (`BlueprintMapLibrary.Map_Values` (`self.EnemiesToKillToWin`)))
  (for _array_element _values
    (if (> _array_element 0)
      (return false)))
  (return true))

(fn `UpdateCurrentGoals`
  (locals (TextArr :type "Array of Text"))
  (bind (_value _returnvalue) (`BlueprintMapLibrary.Map_Find` (`self.EnemiesToKillToWin`) "/Game/RTSGame/Units/Hostile/BP_Guardian.BP_Guardian_C"))
  (bind (_value_2 _returnvalue_2) (`BlueprintMapLibrary.Map_Find` (`self.EnemiesToKillToWin`) "/Game/RTSGame/Units/Hostile/BP_Barbarian.BP_Barbarian_C"))
  (bind (_value_3 _returnvalue_3) (`BlueprintMapLibrary.Map_Find` (`self.EnemiesToKillToWin`) "/Game/RTSGame/Units/Hostile/BP_Mongol.BP_Mongol_C"))
  (`|ExecutionSequence`
    (:`then_0`
      (if (and _returnvalue_3 (> _value_3 0))
        (`KismetArrayLibrary.Array_Add` (`local.TextArr`) (`KismetTextLibrary.Conv_StringToText` (`KismetStringLibrary.Concat_StrStr` "Mongols left: " (`KismetStringLibrary.Conv_IntToString` _value_3))))))
    (:`then_1`
      (if (and _returnvalue_2 (> _value_2 0))
        (`KismetArrayLibrary.Array_Add` (`local.TextArr`) (`KismetTextLibrary.Conv_StringToText` (`KismetStringLibrary.Concat_StrStr` "Barbarians left: " (`KismetStringLibrary.Conv_IntToString` _value_2))))))
    (:`then_2`
      (if (and _returnvalue (> _value 0))
        (`KismetArrayLibrary.Array_Add` (`local.TextArr`) (`KismetTextLibrary.Conv_StringToText` (`KismetStringLibrary.Concat_StrStr` "Guardians left: " (`KismetStringLibrary.Conv_IntToString` _value))))))
    (:`then_3`
      (bind _asbp_hud (cast `/Game/RTSGame/Core/Player/BP_HUD` (`PlayerController.GetHUD` (`GameplayStatics.GetPlayerController` 0))))
      (`/Game/RTSGame/UI/HUD/WBP_HUD.SetCurrentGoals` (`/Game/RTSGame/Core/Player/BP_HUD.HUDWidgetReference` _asbp_hud) (`local.TextArr`)))))

(fn `UserConstructionScript`)