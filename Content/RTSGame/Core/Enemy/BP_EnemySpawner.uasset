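; RTS enemy spawner that periodically spawns random-sized waves of a configured unit at navigable points within its sphere.
; A looping timer drives spawning, capping live units at MaxUnitCount and, for classes in the game mode's EnemiesToKillToWin map, that entry's count.
; Spawned units are tracked until destroyed, when the spawner fires EnemyDestroyed.
; Units with guardian AI controllers receive a reference back to their spawner.
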(event `self.ReceiveBeginPlay`
  (bind _returnvalue (`KismetSystemLibrary.K2_SetTimerDelegate` (delegate `SpawnWave`) (`self.SecondsToSpawnEnemies`) true 0.0 2.0))
  (set `self.SpawnTimer` _returnvalue))

(event `SpawnWave`
  (`self.SpawnEnemy` (`KismetMathLibrary.RandomIntegerInRange` (`self.MinSpawnNumber`) (`self.MaxSpawnNumber`))))

(event `SpawnEnemy`
  (params (EnemiesToSpawn :type Integer :default 1))
  (bind _asgm_rtsgame (cast `/Game/RTSGame/Core/Framework/GM_RTSGame` (`GameplayStatics.GetGameMode`)))
  (for _ (range (+ EnemiesToSpawn 1))
    (if (< (`KismetArrayLibrary.Array_Length` (`self.UnitsSpawned`)) (`self.MaxUnitCount`))
      (bind (_value _returnvalue) (`BlueprintMapLibrary.Map_Find` (`/Game/RTSGame/Core/Framework/GM_RTSGame.EnemiesToKillToWin` _asgm_rtsgame) (`self.ActorToSpawn`)))
      (if (not _returnvalue)
        (bind _returnvalue_2 (`|SpawnActorFromClass` (`self.ActorToSpawn`) (`KismetMathLibrary.MakeTransform` (`self.GetRandomPosition`)) "Undefined" "MultiplyWithRoot" null null :!label _label))
        (`/Engine/EditorBlueprintResources/StandardMacros.IsValid` _returnvalue_2 :!label _label_2
          (:`Is Valid`
            (`self.BindUnit` _returnvalue_2))
          (:`Is Not Valid`
            (`KismetSystemLibrary.Delay` 0.1)
            (goto _label_2)))
        (elif (> _value (`KismetArrayLibrary.Array_Length` (`self.UnitsSpawned`)))
          (goto _label))))))

(event `BindUnit`
  (params (ActorToBind :type "Actor Object Reference"))
  (add `self.OnDestroyed` ActorToBind (delegate `CustomEvent_0`))
  (`KismetArrayLibrary.Array_Add` (`self.UnitsSpawned`) ActorToBind)
  (bind _asai_con_enemy_guardian_unit (cast `/Game/RTSGame/Core/Enemy/AiCon_EnemyGuardianUnit` (`Pawn.GetController` (`Actor.Instigator` ActorToBind))))
  (set `/Game/RTSGame/Core/Enemy/AiCon_EnemyGuardianUnit.SpawnReference` self _asai_con_enemy_guardian_unit))

(event `CustomEvent_0` :!signature `self.OnDestroyed`
  (params (DestroyedActor :type "Actor Object Reference"))
  (`KismetArrayLibrary.Array_RemoveItem` (`self.UnitsSpawned`) DestroyedActor)
  (`self.EnemyDestroyed` DestroyedActor))

(fn `GetRandomPosition`
  (returns (ReturnValue :type "Vector Structure"))
  (bind _randomlocation (`NavigationSystemV1.K2_GetRandomLocationInNavigableRadius` (`self.K2_GetActorLocation` self) (`SphereComponent.GetScaledSphereRadius` (`self.Sphere`)) null null))
  (return (+ _randomlocation (0.0 0.0 100.0))))

(fn `UserConstructionScript`)