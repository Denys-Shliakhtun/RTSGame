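; An actor component for the RTS game that shows a ground-style decal indicator marking its owner as selected.
; On BeginPlay it adds a rotated decal component to the owner, assigns the selection indicator material, hides it, then scales it to IndicatorRadius and applies IndicatorOffset.
; Show and hide events toggle the decal's visibility and keep the IsSelected flag in sync.
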(event `self.ReceiveBeginPlay`
  (bind (_decalsize_x _decalsize_y) (`KismetMathLibrary.BreakVector` (`DecalComponent.DecalSize` (`self.DecalComponentRef`))))
  (bind _returnvalue (/ (`self.IndicatorRadius`) _decalsize_y))
  (bind _returnvalue_2 (`|AddComponentByClass` (`self.GetOwner`) "/Script/Engine.DecalComponent" false (`KismetMathLibrary.MakeTransform` (0.0 0.0 0.0) (struct :`Pitch` 90.0))))
  (bind _output_get (set `self.DecalComponentRef` _returnvalue_2))
  (`DecalComponent.SetDecalMaterial` _output_get "/Game/RTSGame/Core/Common/MI_SelectionIndicator.MI_SelectionIndicator")
  (`self.HideSelectionDecal`)
  (`SceneComponent.SetRelativeScale3D` (`self.DecalComponentRef`) (`KismetMathLibrary.MakeVector` 1.0 _returnvalue _returnvalue))
  (`SceneComponent.K2_SetRelativeLocation` (`self.DecalComponentRef`) (`self.IndicatorOffset`) false false))

(event `ShowSelectionDecal`
  (set `self.IsSelected` true)
  (`SceneComponent.SetHiddenInGame` (`self.DecalComponentRef`) false false))

(event `HideSelectionDecal`
  (set `self.IsSelected` false)
  (`SceneComponent.SetHiddenInGame` (`self.DecalComponentRef`) true false))