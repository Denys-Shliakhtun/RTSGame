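; RTS player controller that drives the camera, unit selection and player orders, and stores gathered resources.
; Keyboard or screen-edge mouse input pans the pawn within boundary corners.
; Clicks and a spawned marquee actor fill the selection list, which updates the HUD info panel.
; Action clicks sphere-overlap the cursor point, then send move, gather, building or hostile-attack orders through interface messages, flagging units as player-ordered.
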(event `self.ReceiveBeginPlay`
  (bind _returnvalue (`|SpawnActorFromClass` "/Game/RTSGame/Core/Player/BP_UnitSelectionMarque.BP_UnitSelectionMarque_C" (`KismetMathLibrary.MakeTransform` (0.0 0.0 0.0)) "Undefined" "MultiplyWithRoot" null null))
  (set `self.SelectionMarqueRef` _returnvalue))

(event `InputAxis|MoveForward`
  (params (AxisValue :type "Float (single-precision)"))
  (bind (_returnvalue_roll _returnvalue_pitch _returnvalue_yaw) (`KismetMathLibrary.BreakRotator` (`self.GetControlRotation`)))
  ;[1 1 1] Camera movement
  (if true
    (`Pawn.AddMovementInput` (`self.K2_GetPawn`) (`KismetMathLibrary.GetForwardVector` (`KismetMathLibrary.MakeRotator` 0.0 0.0 _returnvalue_yaw)) (`KismetMathLibrary.SelectFloat` AxisValue (`self.MouseForwardScale`) (!= AxisValue 0.0)) false)
    (`self.CheckCameraBoundary`)))

(event `InputAxis|MoveRight`
  (params (AxisValue :type "Float (single-precision)"))
  (bind (_returnvalue_roll _returnvalue_pitch _returnvalue_yaw) (`KismetMathLibrary.BreakRotator` (`self.GetControlRotation`)))
  ;[1 1 1] Camera movement
  (`Pawn.AddMovementInput` (`self.K2_GetPawn`) (`KismetMathLibrary.GetRightVector` (`KismetMathLibrary.MakeRotator` 0.0 0.0 _returnvalue_yaw)) (`KismetMathLibrary.SelectFloat` AxisValue (`self.MouseRightScale`) (!= AxisValue 0.0)) false)
  (`self.CheckCameraBoundary`))

(event `InputAxis|MouseMovement`
  (params (AxisValue :type "Float (single-precision)"))
  (bind (_returnvalue_x _returnvalue_y) (`KismetMathLibrary.BreakVector2D` (`WidgetLayoutLibrary.GetViewportSize`)))
  (bind _returnvalue_x_2 (`KismetMathLibrary.BreakVector2D` (`WidgetLayoutLibrary.GetViewportSize`)))
  (bind _viewportedgethreshold (`self.ViewportEdgeThreshold`))
  (bind _viewportedgethreshold_2 (`self.ViewportEdgeThreshold`))
  (bind _returnvalue (/ (`self.GetMousePosition`) _returnvalue_x_2))
  (bind _returnvalue_2 (/ (`.LocationY` (`self.GetMousePosition`)) _returnvalue_y))
  ;[1 1 1] Camera movement
  (set `self.MouseRightScale` (`KismetMathLibrary.SelectFloat` -1.0 (`KismetMathLibrary.SelectFloat` 1.0 0.0 (> _returnvalue (- 1.0 _viewportedgethreshold_2))) (< _returnvalue _viewportedgethreshold_2)))
  (set `self.MouseForwardScale` (`KismetMathLibrary.SelectFloat` 1.0 (`KismetMathLibrary.SelectFloat` -1.0 0.0 (> _returnvalue_2 (- 1.0 _viewportedgethreshold))) (< _returnvalue_2 _viewportedgethreshold))))

(event `AddActorSelectedToList`
  (params (SelectedActor :type "Actor Object Reference"))
  (bind _selectedactors (`self.SelectedActors`))
  (bind _returnvalue (`self.GetComponentByClass` (`|GetArrayItem` _selectedactors) "/Game/RTSGame/Core/Unit/BP_UnitComponent.BP_UnitComponent_C"))
  (if (> (`KismetArrayLibrary.Array_Length` _selectedactors) 0)
    (`/Engine/EditorBlueprintResources/StandardMacros.IsValid` _returnvalue
      (:`Is Valid`
        (clear `/Game/RTSGame/Core/Unit/BP_UnitComponent.OnHPChanged` _returnvalue))
      (:`Is Not Valid`
        _)))
  (`KismetArrayLibrary.Array_Add` _selectedactors SelectedActor)
  (message `/Game/RTSGame/Core/Common/BPI_SelectionEvents.SelectThis` SelectedActor)
  (`self.UpdateHUDInfoPanel`))

(event `DeselectAllActors`
  (bind _selectedactors (`self.SelectedActors`))
  (for _array_element _selectedactors
    (if (`KismetSystemLibrary.DoesImplementInterface` _array_element "/Game/RTSGame/Core/Common/BPI_SelectionEvents.BPI_SelectionEvents_C")
      (message `/Game/RTSGame/Core/Common/BPI_SelectionEvents.DeselectThis` _array_element)))
  (`KismetArrayLibrary.Array_Clear` _selectedactors)
  (`self.UpdateHUDInfoPanel`))

(event `InputAction|MouseSelection`
  (params (Key :type "Key Structure"))
  (:`Pressed`
    (if (`self.IsClickSelected`)
      (set `self.IsClickSelected` false)
      (else
        (`self.DeselectAllActors`)))
    (`self.K2_SetActorLocation` (`self.SelectionMarqueRef`) (`.Location` (`GameplayStatics.BreakHitResult` (`self.GetHitResultUnderCursorByChannel` "TraceTypeQuery1"))) false false)
    (`/Game/RTSGame/Core/Player/BP_UnitSelectionMarque.StartResizingMarquee` (`self.SelectionMarqueRef`)))
  (:`Released`
    (`/Game/RTSGame/Core/Player/BP_UnitSelectionMarque.EndResizingMarquee` (`self.SelectionMarqueRef`))))

(event `InputAction|MouseAction`
  (params (Key :type "Key Structure"))
  (:`Released`
    (if (`KismetArrayLibrary.Array_IsNotEmpty` (`self.SelectedActors`))
      (`self.DoAction` (`.Location` (`GameplayStatics.BreakHitResult` (`self.GetHitResultUnderCursorByChannel` "TraceTypeQuery1"))) (`self.SelectedActors`)))))

(event `DoAction`
  (params (AimLocation :type "Vector Structure") (ActorsToPerformAction :type "Array of Actor Object Reference"))
  (bind (_bblockinghit _binitialoverlap _time _distance _location) (`GameplayStatics.BreakHitResult` (`self.GetHitResultUnderCursorByChannel` "TraceTypeQuery1")))
  (for _array_element ActorsToPerformAction
    (bind _returnvalue (`self.GetComponentByClass` _array_element "/Game/RTSGame/Core/Unit/BP_UnitComponent.BP_UnitComponent_C"))
    (if (`KismetSystemLibrary.IsValid` _returnvalue)
      (set `/Game/RTSGame/Core/Unit/BP_UnitComponent.HasOrderFromPlayer` true _returnvalue)))
  (bind _outactors (`KismetSystemLibrary.SphereOverlapActors` AimLocation 100.0 (`|MakeArray` "ObjectTypeQuery2" "ObjectTypeQuery3" :!type "EObjectTypeQuery Enum")))
  (if (`KismetArrayLibrary.Array_IsEmpty` _outactors)
    ;[1 1 1] Unit Movement
    (for _array_element_2 ActorsToPerformAction
      (if (`KismetSystemLibrary.DoesImplementInterface` _array_element_2 "/Game/RTSGame/Core/Unit/BPI_UnitActions.BPI_UnitActions_C")
        (message `/Game/RTSGame/Core/Unit/BPI_UnitActions.MoveToThisLocation` _array_element_2 _location)
        (`NiagaraFunctionLibrary.SpawnSystemAtLocation` "/Game/RTSGame/Core/Player/NS_ClickIndicator.NS_ClickIndicator" _location)))
    (else
      (for _array_element_3 ActorsToPerformAction
        (if (`KismetSystemLibrary.DoesImplementInterface` _array_element_3 "/Game/RTSGame/Core/Unit/BPI_UnitActions.BPI_UnitActions_C")
          (bind _output (`|GetArrayItem` _outactors))
          (if (`KismetSystemLibrary.IsValid` (`self.GetComponentByClass` _output "/Game/RTSGame/Core/Resource/BP_ResourceComponent.BP_ResourceComponent_C"))
            (message `/Game/RTSGame/Core/Unit/BPI_UnitActions.GatherThisResource` _array_element_3 _output)
            (elif (`KismetSystemLibrary.IsValid` (`self.GetComponentByClass` _output "/Game/RTSGame/Core/Building/BP_BuildingComponent.BP_BuildingComponent_C"))
              (message `/Game/RTSGame/Core/Unit/BPI_UnitActions.InteractWithBuilding` _array_element_3 _output)
              (else
                (bind _returnvalue_2 (`self.GetComponentByClass` _output "/Game/RTSGame/Core/Unit/BP_UnitComponent.BP_UnitComponent_C"))
                (if (`KismetSystemLibrary.IsValid` _returnvalue_2)
                  (if (`|EnumEquality` (`/Game/RTSGame/Core/Unit/BP_UnitComponent.TeamAttitude` _returnvalue_2) "Hostile")
                    (message `/Game/RTSGame/Core/Unit/BPI_UnitActions.AttackThisActor` _array_element_3 _output)))))))))))

(event `ResumeUnitActions`
  (params (ActorAndLocation :type "Array of /Game/RTSGame/UI/Menus/SaveGame/S_UnitReference Structure"))
  (if (`KismetArrayLibrary.Array_IsNotEmpty` ActorAndLocation)
    (for _array_element ActorAndLocation
      (`self.DoAction` (`.Target_5_9C2B625944F32C70961CE4B61DD7B736` (break `/Game/RTSGame/UI/Menus/SaveGame/S_UnitReference` _array_element)) (`|MakeArray` (break `/Game/RTSGame/UI/Menus/SaveGame/S_UnitReference` _array_element))))))

(event `/Game/RTSGame/Core/Common/BPI_SelectionEvents.SelectThisActor`
  (params (ActorSelected :type "Actor Object Reference"))
  (`self.AddActorSelectedToList` ActorSelected))

(event `/Game/RTSGame/Core/Common/BPI_SelectionEvents.DeselectThisActor`
  (params (ActorDeselected :type "Actor Object Reference"))
  (`self.ActorDeselection` ActorDeselected))

(event `/Game/RTSGame/Core/Common/BPI_SelectionEvents.ClickSelectThisActor`
  (params (ActorSelected :type "Actor Object Reference"))
  (set `self.IsClickSelected` true)
  (`self.DeselectAllActors`)
  (`/Game/RTSGame/Core/Common/BPI_SelectionEvents.SelectThisActor` ActorSelected))

(fn `ActorDeselection`
  (params (ActorDeselected :type "Actor Object Reference"))
  (bind _returnvalue (`KismetArrayLibrary.Array_RemoveItem` (`self.SelectedActors`) ActorDeselected))
  (if (and _returnvalue (`KismetSystemLibrary.DoesImplementInterface` ActorDeselected "/Game/RTSGame/Core/Common/BPI_SelectionEvents.BPI_SelectionEvents_C"))
    (message `/Game/RTSGame/Core/Common/BPI_SelectionEvents.DeselectThis` ActorDeselected)
    (`self.UpdateHUDInfoPanel`)))

(fn `CheckCameraBoundary`
  (bind _returnvalue (`self.K2_GetPawn`))
  (bind (_toprightboundary_x _toprightboundary_y) (`KismetMathLibrary.BreakVector` (`self.TopRightBoundary`)))
  (bind (_bottomleftboundary_x _bottomleftboundary_y) (`KismetMathLibrary.BreakVector` (`self.BottomLeftBoundary`)))
  (bind (_returnvalue_x _returnvalue_y _returnvalue_z) (`KismetMathLibrary.BreakVector` (`self.K2_GetActorLocation` _returnvalue)))
  (bind (_returnvalue_x_2 _returnvalue_y_2 _returnvalue_z_2) (`KismetMathLibrary.BreakVector` (`self.K2_GetActorLocation` (`self.K2_GetPawn`))))
  (`|ExecutionSequence`
    (:`then_0`
      (if (> _returnvalue_x _toprightboundary_x)
        (`self.K2_SetActorLocation` _returnvalue (`KismetMathLibrary.MakeVector` _toprightboundary_x _returnvalue_y _returnvalue_z) false false)))
    (:`then_1`
      (if (> _returnvalue_y _toprightboundary_y)
        (`self.K2_SetActorLocation` _returnvalue (`KismetMathLibrary.MakeVector` _returnvalue_x _toprightboundary_y _returnvalue_z) false false)))
    (:`then_2`
      (if (< _returnvalue_x_2 _bottomleftboundary_x)
        (`self.K2_SetActorLocation` _returnvalue (`KismetMathLibrary.MakeVector` _bottomleftboundary_x _returnvalue_y_2 _returnvalue_z_2) false false)))
    (:`then_3`
      (if (< _returnvalue_y_2 _bottomleftboundary_y)
        (`self.K2_SetActorLocation` _returnvalue (`KismetMathLibrary.MakeVector` _returnvalue_x_2 _bottomleftboundary_y _returnvalue_z_2) false false)))))

(fn `GetTeamAttitude`
  (returns (TeamAttitude :type "ETeamAttitude Enum"))
  (return "Friendly"))

(fn `ReceiveResources`
  (params (Type :type "/Game/RTSGame/Core/Resource/E_ResourceType Enum" :default "NewEnumerator0") (Amount :type Integer))
  (bind _type (`local.Type`))
  (`|ExecutionSequence`
    (:`then_0`
      (if (`BlueprintMapLibrary.Map_Contains` (`self.StoredResources`) Type)
        (`BlueprintMapLibrary.Map_Add` (`self.StoredResources`) (`local.Type`) (+ (`BlueprintMapLibrary.Map_Find` (`self.StoredResources`) (`local.Type`)) (`local.Amount`)))
        (else
          (`BlueprintMapLibrary.Map_Add` (`self.StoredResources`) (`local.Type`) (`local.Amount`)))))
    (:`then_1`
      (bind _asbp_hud (cast `/Game/RTSGame/Core/Player/BP_HUD` (`self.GetHUD`)))
      (bind _hudwidgetreference (`/Game/RTSGame/Core/Player/BP_HUD.HUDWidgetReference` _asbp_hud))
      (`/Engine/EditorBlueprintResources/StandardMacros.IsValid` _hudwidgetreference
        (:`Is Valid`
          (`/Game/RTSGame/UI/HUD/WBP_HUD.UpdateResourceValue` _hudwidgetreference _type (`BlueprintMapLibrary.Map_Find` (`self.StoredResources`) _type)))))))

(fn `UpdateHUDInfoPanel`
  (bind _asbp_hud (cast `/Game/RTSGame/Core/Player/BP_HUD` (`self.GetHUD`)))
  (`/Game/RTSGame/UI/HUD/WBP_HUD.UpdateInfoPanel` (`/Game/RTSGame/Core/Player/BP_HUD.HUDWidgetReference` _asbp_hud) (`self.SelectedActors`)))

(fn `UserConstructionScript`)