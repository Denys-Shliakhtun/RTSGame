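; BP_Mongol is a hostile Mongol unit Blueprint for the RTS game, with only a small amount of logic of its own.
; Its construction script tints the unit semi-transparent red through SetColorOfUnit.
; When StopAttack fires, it casts its controller to AiCon_EnemyMongolUnit and calls FindTargetToAttack, leaving target selection to the AI controller.
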(event `self.StopAttack`
  (bind _asai_con_enemy_mongol_unit (cast `/Game/RTSGame/Core/Enemy/AiCon_EnemyMongolUnit` (`self.GetController`)))
  (`/Game/RTSGame/Core/Enemy/AiCon_EnemyMongolUnit.FindTargetToAttack` _asai_con_enemy_mongol_unit))

(fn `UserConstructionScript`
  (`self.SetColorOfUnit` (struct :`R` 1.0 :`G` 0.050213 :`A` 0.5)))