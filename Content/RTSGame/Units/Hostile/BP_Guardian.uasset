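; BP_Guardian is a hostile RTS unit, tinted translucent red in its construction script, that alerts its AI to player-side units it notices.
; PawnNoticed stores a valid pawn and passes it to PawnObserved, which checks that it is a BP_Unit whose BP_UnitComponent has a Friendly team attitude.
; Matching units are forwarded to AiCon_EnemyGuardianUnit through OnEnemyObserved, leaving the response to that controller.
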(event `self.PawnNoticed`
  (params (InputPin :type "Pawn Object Reference"))
  (`/Engine/EditorBlueprintResources/StandardMacros.IsValid` InputPin
    (:`Is Valid`
      (bind _output_get (set `self.Pawn` InputPin))
      (`self.PawnObserved` _output_get))))

(fn `PawnObserved`
  (params (InputPin :type "Pawn Object Reference"))
  (bind _asai_con_enemy_guardian_unit (cast `/Game/RTSGame/Core/Enemy/AiCon_EnemyGuardianUnit` (`self.GetController`)))
  (bind _asbp_unit (cast `/Game/RTSGame/Core/Unit/BP_Unit` InputPin))
  (if (`|EnumEquality` (`/Game/RTSGame/Core/Unit/BP_UnitComponent.TeamAttitude` (`self.GetComponentByClass` _asbp_unit "/Game/RTSGame/Core/Unit/BP_UnitComponent.BP_UnitComponent_C")) "Friendly")
    (`/Game/RTSGame/Core/Enemy/AiCon_EnemyGuardianUnit.OnEnemyObserved` _asai_con_enemy_guardian_unit InputPin)))

(fn `UserConstructionScript`
  (`self.SetColorOfUnit` (struct :`R` 1.0 :`G` 0.050213 :`A` 0.5)))